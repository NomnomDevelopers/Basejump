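; PortalSpawn is an actor that randomly spawns MonsterSpawner actors at its Billboard's location and rotation.
; From BeginPlay, a looping random roll gives about a three-in-ten chance to spawn, ignoring collision.
; A failed roll or a valid new spawner leads to a one-minute delay before rolling again, while an invalid spawner reference is rechecked every second.
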(event EventBeginPlay
  (bind _billboard (Variables|Default|GetBillboard))
  (if (<= (Math|Random|RandomInteger 10) 2) :!label _label
    (bind _returnvalue (Game|SpawnActorfromClass "/Game/Blueprints/MonsterSpawner.MonsterSpawner_C" (Math|Transform|MakeTransform (Transformation|GetWorldLocation _billboard) (Transformation|GetWorldRotation _billboard) "1,1,1") "AlwaysSpawn" 0 0))
    (if (Utilities|IsValid _returnvalue) :!label _label_2
      _
      (else
        (Utilities|FlowControl|Delay 1.0)
        (goto _label_2))))
  (Utilities|FlowControl|Delay 6e+01)
  (goto _label))

(event EventActorBeginOverlap
  (params (OtherActor :type Actor%20Object%20Reference)))

(event EventTick
  (params (DeltaSeconds :type Float%20%28single-precision%29)))

(fn ConstructionScript)