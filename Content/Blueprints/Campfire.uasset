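; Campfire actor that heals nearby allowed actors while its own Health burns down over time.
; HealDistance overlaps maintain Targets, and every tick applies negative damage to AllowedToHeal classes, plus slight damage to the fire itself.
; AnyDamage updates Health and toggles the flame particles, hiding them at zero.
; While lit but low, it feeds itself by damaging a random AllowedToBurn target in range and applying negative damage to itself.
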(event OnComponentBeginOverlap(HealDistance)
  (params (OtherActor :type Actor%20Object%20Reference) (OtherComp :type Primitive%20Component%20Object%20Reference) (OtherBodyIndex :type Integer) (bFromSweep :type Boolean) (SweepResult :type Hit%20Result%20Structure%20%28by%20ref%29))
  (Utilities|Array|Add (Variables|Default|GetTargets) OtherActor))

(event OnComponentEndOverlap(HealDistance)
  (params (OtherActor :type Actor%20Object%20Reference) (OtherComp :type Primitive%20Component%20Object%20Reference) (OtherBodyIndex :type Integer))
  (Utilities|Array|RemoveItem (Variables|Default|GetTargets) OtherActor))

(event Custom|HealTest
  (Utilities|IsValid (Utilities|Array|Get(acopy) (Variables|Default|GetTargets))
    (:Is%20Valid
      (for _array_element (Variables|Default|GetTargets)
        (if (Utilities|Array|ContainsItem (Variables|Default|GetAllowedToHeal) (Utilities|GetClass _array_element))
          (Game|Damage|ApplyDamage _array_element -12.0 0 self "/Script/Engine.DamageType"))))))

(event Custom|TickingHP
  (bind _self self)
  ;[1 1 1] TickingHP
  (Game|Damage|ApplyDamage _self (* (Utilities|Time|GetWorldDeltaSeconds) 0.33) 0 _self "/Script/Engine.DamageType"))

(event Custom|BurneeDestroyed
  (params (RemoveFromArray :type Actor%20Object%20Reference))
  (Utilities|Array|RemoveItem (Variables|Default|GetTargets) RemoveFromArray))

(event Custom|PutOutFire
  (Rendering|SetVisibility (Variables|Default|GetParticleSystem) false false))

(event Custom|StealHpFromBurnee
  (Utilities|IsValid (Utilities|Array|Get(acopy) (Variables|Default|GetTargets))
    (:Is%20Valid
      (Utilities|Array|Clear (Variables|Default|GetBurnTargets))
      (for _array_element (Variables|Default|GetTargets)
        (if (Utilities|Array|ContainsItem (Variables|Default|GetAllowedToBurn) (Utilities|GetClass _array_element))
          (Utilities|Array|Add (Variables|Default|GetBurnTargets) _array_element)))
      (Utilities|IsValid (Utilities|Array|Get(acopy) (Variables|Default|GetBurnTargets))
        (:Is%20Valid
          (Game|Damage|ApplyDamage (Utilities|Array|Get(acopy) (Variables|Default|GetBurnTargets) (Math|Random|RandomIntegerinRange 0 (- (Utilities|Array|Length (Variables|Default|GetBurnTargets)) 1))) 3e+01 0 self "/Script/Engine.DamageType")
          (Game|Damage|ApplyDamage self -3e+01 0 0 "/Script/Engine.DamageType"))))))

(event Custom|StartFire
  (Rendering|SetVisibility (Variables|Default|GetParticleSystem) true false))

(event EventTick
  (params (DeltaSeconds :type Float%20%28single-precision%29))
  (CallFunction|HealTest)
  (CallFunction|TickingHP))

(event Game|Damage|EventAnyDamage
  (params (Damage :type Float%20%28single-precision%29) (DamageType :type Damage%20Type%20Object%20Reference) (InstigatedBy :type Controller%20Object%20Reference) (DamageCauser :type Actor%20Object%20Reference))
  (Variables|Default|SetHealth (Math|Float|Max(Float) (- (Variables|Default|GetHealth) Damage) 0.0))
  (if (<= (Variables|Default|GetHealth) 0.0)
    (CallFunction|PutOutFire)
    (else
      (CallFunction|StartFire)
      (if (< (Variables|Default|GetHealth) 1.2e+02)
        (CallFunction|StealHpfromBurnee)))))

(fn ConstructionScript)