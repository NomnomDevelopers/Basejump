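; Hex tile actor that randomly shifts position and spawns bullet pickups, changing material to show its state.
; A BeginPlay loop randomly turns it red, waits, then moves it in two stepped runs, both along Direction (Reverse is unused), using Time array length as step counter.
; A delayed Tick loop occasionally turns it purple and spawns a short-lived BulletPickup at the Box.
; Overlaps swap the material and restore the default after a delay.
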(event OnComponentBeginOverlap(Box)
  (params (OtherActor :type Actor%20Object%20Reference) (OtherComp :type Primitive%20Component%20Object%20Reference) (OtherBodyIndex :type Integer) (bFromSweep :type Boolean) (SweepResult :type Hit%20Result%20Structure%20%28by%20ref%29))
  (Rendering|Material|SetMaterial (Variables|Default|GetStaticMesh) 1 "/Game/ThirdPersonBP/Assets/Hex/catfur.catfur"))

(event Collision|EventActorBeginOverlap
  (params (OtherActor :type Actor%20Object%20Reference))
  (Utilities|FlowControl|Delay 0.5)
  (switch int 0
    (:0
      (Rendering|Material|SetMaterial (Variables|Default|GetStaticMesh) 1 "/Game/ThirdPersonBP/Assets/Hex/02_-_Default.02_-_Default"))))

(event EventBeginPlay
  (bind _returnvalue (Utilities|Time|GetWorldDeltaSeconds))
  (bind _staticmesh (Variables|Default|GetStaticMesh))
  (bind _speed (Variables|Default|GetSpeed))
  (bind _direction (Variables|Default|GetDirection))
  (bind _time (Variables|Default|GetTime))
  (bind _time_2 (Variables|Default|GetTime))
  (bind _returnvalue_2 (Transformation|GetWorldTransform _staticmesh))
  (bind _returnvalue_3 (Math|Vector|Normalize _direction))
  (bind _returnvalue_4 (* _returnvalue _speed))
  (bind (_location _rotation _scale) (Math|Transform|BreakTransform _returnvalue_2))
  (bind _returnvalue_5 (* _returnvalue_3 _returnvalue_4))
  (bind _returnvalue_6 (+ _returnvalue_5 _location))
  (bind _returnvalue_7 (Math|Transform|MakeTransform _returnvalue_6 _rotation _scale))
  (Utilities|FlowControl|Delay 5.0 :!label _label)
  (if (<= (Math|Random|RandomInteger 10) 5)
    (Rendering|Material|SetMaterial _staticmesh 1 "/Game/ThirdPersonBP/Assets/Hex/REDLIGHT.REDLIGHT")
    (Utilities|FlowControl|Delay 5.0)
    (Transformation|SetActorTransform _returnvalue_7 :!label _label_2)
    (if (== (Math|Conversions|ToFloat(Integer) (Utilities|Array|Length _time_2)) 5e+01)
      (Utilities|Array|Clear _time_2)
      (Transformation|SetActorTransform _returnvalue_7 :!label _label_3)
      (if (== (Math|Conversions|ToFloat(Integer) (Utilities|Array|Length _time)) 5e+01)
        (Rendering|Material|SetMaterial (Variables|Default|GetStaticMesh) 1 "/Game/ThirdPersonBP/Assets/Hex/02_-_Default.02_-_Default")
        (Utilities|Array|Clear (Variables|Default|GetTime))
        (goto _label)
        (else
          (Utilities|FlowControl|Delay 0.01)
          (Utilities|Array|Add _time 0.0)
          (goto _label_3)))
      (else
        (Utilities|FlowControl|Delay 0.01)
        (Utilities|Array|Add _time_2 0.0)
        (goto _label_2)))
    (else
      (goto _label))))

(event EventActorBeginOverlap
  (params (OtherActor :type Actor%20Object%20Reference)))

(event EventTick
  (params (DeltaSeconds :type Float%20%28single-precision%29))
  (Utilities|FlowControl|Delay 6.0 :!label _label)
  (if (<= (Math|Random|RandomInteger 100) 5)
    (Rendering|Material|SetMaterial (Variables|Default|GetStaticMesh) 1 "/Game/ThirdPersonBP/Assets/Hex/Purple.Purple")
    (bind _returnvalue (Game|SpawnActorfromClass "/Game/Blueprints/BulletPickup.BulletPickup_C" (Math|Conversions|ToTransform(Vector) (Transformation|GetWorldLocation (Variables|Default|GetBox))) "AdjustIfPossibleButAlwaysSpawn" 0 0))
    (Actor|SetLifeSpan _returnvalue 1e+01)
    (goto _label)
    (else
      (goto _label))))

(fn ConstructionScript)