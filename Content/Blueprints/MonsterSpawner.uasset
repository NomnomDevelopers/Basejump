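; MonsterSpawner is a portal-like spawner actor that spawns one monster at its own transform shortly after play begins.
; BeginPlay waits briefly, then calls SpawnMonsters, which spawns only the first class in ListOfSpawnableMonsters.
; Tick spins four portal components with fixed per-frame local rotations at differing speeds, axes and directions, so the animation speed depends on frame rate.
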(event Custom|SpawnMonsters
  (Game|SpawnActorfromClass (Utilities|Array|Get(acopy) (Variables|Default|GetListOfSpawnableMonsters)) (Transformation|GetActorTransform) "Undefined" 0 0))

(event EventBeginPlay
  (Utilities|FlowControl|Delay 0.2)
  (CallFunction|SpawnMonsters))

(event EventTick
  (params (DeltaSeconds :type Float%20%28single-precision%29))
  (Transformation|AddLocalRotation (Variables|Default|GetStaticMesh) (Math|Rotator|MakeRotator 0.5 0.0 0.0) false false)
  (Transformation|AddLocalRotation (Variables|Default|GetStaticMesh1) (Math|Rotator|MakeRotator 0.0 0.0 -0.2) false false)
  (Transformation|AddLocalRotation (Variables|Default|Getportal_Object) (Math|Rotator|MakeRotator -0.2 0.0 0.0) false false)
  (Transformation|AddLocalRotation (Variables|Default|Getportal_Object002) (Math|Rotator|MakeRotator 0.1 0.0 0.0) false false))

(fn ConstructionScript)