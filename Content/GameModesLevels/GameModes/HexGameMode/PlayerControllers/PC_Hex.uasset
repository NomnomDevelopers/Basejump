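; PC_Hex is the player controller in the HexGameMode folder, responsible for the player's multiplayer HUD.
; ClientPostLogin calls SetupGameHUD, which creates a W_MPHUD widget only for a local controller, stores it and adds it to the viewport.
; The event then casts the game mode to HexGameMode, with nothing following the cast.
; EndPlay removes the HUD widget from its parent.
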(event Custom|ClientPostLogin
  (CallFunction|SetupGameHUD)
  (Utilities|Casting|CastToHexGameMode (Game|GetGameMode)))

(event EventEndPlay
  (params (EndPlayReason :type EEndPlayReason%20Enum :default "Destroyed"))
  (Widget|RemovefromParent (Variables|Default|Getw_HUD)))

(fn ConstructionScript)

(fn SetupGameHUD
  (if (Pawn|IsLocalPlayerController)
    (bind _returnvalue (UserInterface|CreateWidget "/Game/GameModesLevels/GameModes/HexGameMode/Widgets/W_MPHUD.W_MPHUD_C" self))
    (bind _output_get (Variables|Default|Setw_HUD _returnvalue))
    (UserInterface|Viewport|AddtoViewport _output_get 0)))